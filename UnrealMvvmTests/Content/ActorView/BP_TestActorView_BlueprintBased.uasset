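; BP_TestActorView_BlueprintBased is a test actor that exercises Blueprint access to a view model from an actor view, for C++ tests.
; It records the IntValue property on change notifications, plus old, new and getter-returned view models when the view model changes.
; Custom events write IntValue back, either from a parameter or as a constant the tests expect, and a function returns a view model property value.
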(event `self.SetValueToViewModel`
  (params (NewValue :type Integer))
  (`|SetViewModelPropertyValue` NewValue))

(event `self.SetValueToViewModelConstant`
  (`|SetViewModelPropertyValue` 123) ; Value 123 is expected by c++ tests
)

(fn `GetValueFromViewModel`
  (returns (ReturnValue :type Integer))
  (return (`|GetViewModelPropertyValue` null)))

(fn `UserConstructionScript`)